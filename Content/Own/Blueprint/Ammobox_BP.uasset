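; Ammo box actor for motion-controller play that dispenses Ammo_BP while it is grabbed.
; GrabComponent events track first and second grabs, and Grab and Release events store or clear the MotionController.
; On box overlap during either grab, it looks up an existing Ammo_BP, spawns another at its own transform, then attaches the existing one, not the spawned one, to that controller.
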(event OnComponentBeginOverlap(Box)
  (params (OverlappedComponent :type Primitive%20Component%20Object%20Reference) (OtherActor :type Actor%20Object%20Reference) (OtherComp :type Primitive%20Component%20Object%20Reference) (OtherBodyIndex :type Integer) (bFromSweep :type Boolean) (SweepResult :type Hit%20Result%20Structure%20%28by%20ref%29))
  (if (or (Variables|Default|Getsecondgrab) (Variables|Default|Getfirstgrab%20))
    (bind _returnvalue (Actor|GetActorOfClass "/Game/Own/Blueprint/Ammo_BP.Ammo_BP_C"))
    (bind _asammo_bp (Utilities|Casting|CastToAmmo_BP _returnvalue))
    (Game|SpawnActorfromClass "/Game/Own/Blueprint/Ammo_BP.Ammo_BP_C" (Transformation|GetActorTransform) "Undefined" "MultiplyWithRoot" 0 0)
    (Transformation|AttachComponentToComponent _asammo_bp (Variables|Default|GetMotion%20Controller) "None" "KeepRelative" "KeepRelative" "KeepRelative" true)))

(event FirstonGrabbed(GrabComponent)
  (params (MotionController :type Motion%20Controller%20Component%20Object%20Reference) (MotionControllerAim :type Motion%20Controller%20Component%20Object%20Reference))
  (Variables|Default|Setfirstgrab%20 true))

(event FirstonDropped(GrabComponent)
  (Variables|Default|Setfirstgrab%20 false))

(event SecondonGrabbed(GrabComponent)
  (params (MotionController :type Motion%20Controller%20Component%20Object%20Reference) (MotionControllerAim :type Motion%20Controller%20Component%20Object%20Reference))
  (Variables|Default|Setsecondgrab true))

(event SecondonDropped(GrabComponent)
  (Variables|Default|Setsecondgrab false))

(event EventBeginPlay)

(event Collision|EventActorBeginOverlap
  (params (OtherActor :type Actor%20Object%20Reference)))

(event EventTick
  (params (DeltaSeconds :type Float%20%28single-precision%29)))

(event EventGrab
  (params (MotionController :type Motion%20Controller%20Component%20Object%20Reference))
  (Variables|Default|SetMotion%20Controller MotionController))

(event EventRelease
  (params (MotionController :type Motion%20Controller%20Component%20Object%20Reference))
  (if (== (Variables|Default|GetMotion%20Controller) MotionController)
    (Variables|Default|SetMotion%20Controller 0)))

(fn ConstructionScript)