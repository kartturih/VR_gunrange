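; BP_TargetSphere is a target-shooting minigame actor with four spheres, one randomly highlighted red as the active target after StartTargets.
; Hitting the red sphere adds a point and picks a different one by re-rolling; other hits subtract a point.
; Both update the score widget, reached through its spawner actor.
; At 25 points it destroys itself, flags the timer widget as won, resets BP_ButtonL and spawns BP_Restart.
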(event Custom|StartTargets
  (bind _output_get (Variables|Default|SetTargets (Utilities|Array|MakeArray (Variables|Default|GetSphere) (Variables|Default|GetSphere1) (Variables|Default|GetSphere2) (Variables|Default|GetSphere3))))
  (bind _output_get_2 (Variables|Default|SetIsRed (.OutItem (Utilities|Array|Random _output_get))))
  (Rendering|Material|SetMaterial _output_get_2 0 "/Game/Own/Material/M_Red.M_Red")
  (Development|PrintString (Utilities|GetDisplayName _output_get_2)))

(event Collision|EventHit
  (params (MyComp :type Primitive%20Component%20Object%20Reference) (Other :type Actor%20Object%20Reference) (OtherComp :type Primitive%20Component%20Object%20Reference) (bSelfMoved :type Boolean) (HitLocation :type Vector :default "0, 0, 0") (HitNormal :type Vector :default "0, 0, 0") (NormalImpulse :type Vector :default "0, 0, 0") (Hit :type Hit%20Result%20Structure%20%28by%20ref%29))
  (if (== MyComp (Variables|Default|GetIsRed))
    (for _array_element (Variables|Default|GetTargets)
      (Rendering|Material|SetMaterial _array_element 0 "/Game/FPWeapon/Materials/BaseMaterial.BaseMaterial"))
    (bind _output_get (Variables|Default|SetIsRedNew (.OutItem (Utilities|Array|Random (Variables|Default|GetTargets)))))
    (if (!= _output_get (Variables|Default|GetIsRed))
      _
      (else
        (while (== _output_get (Variables|Default|GetIsRed))
          (Variables|Default|SetIsRedNew (.OutItem (Utilities|Array|Random (Variables|Default|GetTargets)))))))
    (Rendering|Material|SetMaterial _output_get 0 "/Game/Own/Material/M_Red.M_Red")
    (Variables|Default|SetIsRed _output_get)
    (bind _returnvalue (Actor|GetActorOfClass "/Game/Own/Widgets/BP_Spawn_ScoreCounter.BP_Spawn_ScoreCounter_C"))
    (bind _aswbp_score_counter (Utilities|Casting|CastToWBP_ScoreCounter (UserInterface|GetWidget (Variables|/Game/Own/Widgets/BP_Spawn_ScoreCounter.BP_Spawn_ScoreCounter_C|GetWidget _returnvalue))))
    (Default|Counter+ _aswbp_score_counter)
    (bind _output_get_2 (Variables|Default|SetScoreCounter (+ (Variables|Default|GetScoreCounter) 1)))
    (Development|PrintString (Utilities|String|ToString(Integer) _output_get_2))
    (if (== (Variables|Default|GetScoreCounter) 25)
      (for _array_element_2 (Variables|Default|GetTargets)
        (Actor|DestroyActor))
      (bind _returnvalue_2 (Actor|GetActorOfClass "/Game/Own/Widgets/BP_Spawn_TimeCounter.BP_Spawn_TimeCounter_C"))
      (bind _aswbp_time_counter (Utilities|Casting|CastToWBP_TimeCounter (UserInterface|GetWidget (Variables|/Game/Own/Widgets/BP_Spawn_TimeCounter.BP_Spawn_TimeCounter_C|GetWidget _returnvalue_2))))
      (Variables|/Game/Own/Widgets/WBP_TimeCounter.WBP_TimeCounter_C|SetGameWon _aswbp_time_counter true)
      (bind _returnvalue_3 (Actor|GetActorOfClass "/Game/Own/Blueprint/BP_ButtonL.BP_ButtonL_C"))
      (Default|ResetButton _returnvalue_3)
      (Game|SpawnActorfromClass "/Game/Own/Blueprint/BP_Restart.BP_Restart_C" (Variables|Default|GetSpawnRestartLocation) "Undefined" "MultiplyWithRoot" 0 0))
    (else
      (bind _output_get_3 (Variables|Default|SetScoreCounter (- (Variables|Default|GetScoreCounter) 1)))
      (Development|PrintString (Utilities|String|ToString(Integer) _output_get_3))
      (bind _returnvalue_4 (Actor|GetActorOfClass "/Game/Own/Widgets/BP_Spawn_ScoreCounter.BP_Spawn_ScoreCounter_C"))
      (bind _aswbp_score_counter_2 (Utilities|Casting|CastToWBP_ScoreCounter (UserInterface|GetWidget (Variables|/Game/Own/Widgets/BP_Spawn_ScoreCounter.BP_Spawn_ScoreCounter_C|GetWidget _returnvalue_4))))
      (Default|Counter- _aswbp_score_counter_2))))

(fn ConstructionScript)