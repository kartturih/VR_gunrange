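; Target-shooting minigame actor with four spheres that slide back and forth along Y, one highlighted red as the target.
; BeginPlay starts ping-pong timeline lerps per sphere, two running in the opposite direction; StartMovingTargets picks the first red sphere.
; Hitting red raises the score and re-rolls a different target; other hits lower it, both calling the score widget.
; At 15 points it flags the timer widget as won, spawns BP_Restart and destroys itself.
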(event Custom|CustomEvent_2
  (bind _sphere3 (Variables|Default|GetSphere3))
  (bind _returnvalue (Transformation|GetWorldLocation _sphere3))
  ;[1 1 1] Comment
  (bind _output_get (Variables|Default|SetStart3 (Math|Vector|MakeVector (.x _returnvalue) (.y _returnvalue) (.z _returnvalue))))
  (Development|PrintString (Utilities|String|ToString(Vector) _output_get))
  (Variables|Default|SetEnd3 (Math|Vector|MakeVector (.x _returnvalue) 6.7e+02 (.z _returnvalue)))
  (bind _move (Timeline|Timeline_5 PlayFromStart)
    (:Update
      (Transformation|SetWorldLocation (Variables|Default|GetSphere3) (Math|Vector|Lerp(Vector) (Variables|Default|GetStart3) (Variables|Default|GetEnd3) _move) false false))
    (:Finished
      (bind _move_2 (Timeline|Timeline_6 ReverseFromEnd)
        (:Update
          (Transformation|SetWorldLocation (Variables|Default|GetSphere3) (Math|Vector|Lerp(Vector) (Variables|Default|GetStart3) (Variables|Default|GetEnd3) _move_2) false false))
        (:Finished
          (Timeline|Timeline_5 PlayFromStart))))))

(event Custom|StartMovingTargets
  ;[1 1 1] Starts Targets
  (bind _output_get (Variables|Default|SetTargets (Utilities|Array|MakeArray (Variables|Default|GetSphere) (Variables|Default|GetSphere1) (Variables|Default|GetSphere2) (Variables|Default|GetSphere3))))
  (bind _output_get_2 (Variables|Default|SetIsRed (.OutItem (Utilities|Array|Random _output_get))))
  (Rendering|Material|SetMaterial _output_get_2 0 "/Game/Own/Material/M_Red.M_Red")
  (Development|PrintString (Utilities|GetDisplayName _output_get_2)))

(event Custom|Moving%20Targets
  (bind _sphere1 (Variables|Default|GetSphere1))
  (bind _returnvalue (Transformation|GetWorldLocation _sphere1))
  ;[1 1 1] Moving Targets
  (bind _output_get (Variables|Default|SetStart (Math|Vector|MakeVector (.x _returnvalue) (.y _returnvalue) (.z _returnvalue))))
  (Development|PrintString (Utilities|String|ToString(Vector) _output_get))
  (Variables|Default|SetEnd (Math|Vector|MakeVector (.x _returnvalue) 6.7e+02 (.z _returnvalue)))
  (bind _move (Timeline|Timeline PlayFromStart)
    (:Update
      (Transformation|SetWorldLocation (Variables|Default|GetSphere1) (Math|Vector|Lerp(Vector) (Variables|Default|GetStart) (Variables|Default|GetEnd) _move) false false))
    (:Finished
      (bind _move_2 (Timeline|Timeline_0 ReverseFromEnd)
        (:Update
          (Transformation|SetWorldLocation (Variables|Default|GetSphere1) (Math|Vector|Lerp(Vector) (Variables|Default|GetStart) (Variables|Default|GetEnd) _move_2) false false))
        (:Finished
          (Timeline|Timeline PlayFromStart))))))

(event Custom|CustomEvent
  (bind _sphere (Variables|Default|GetSphere))
  (bind _returnvalue (Transformation|GetWorldLocation _sphere))
  ;[1 1 1] Comment
  (bind _output_get (Variables|Default|SetStart2 (Math|Vector|MakeVector (.x _returnvalue) 6.7e+02 (.z _returnvalue))))
  (Development|PrintString (Utilities|String|ToString(Vector) _output_get))
  (Variables|Default|SetEnd2 (Math|Vector|MakeVector (.x _returnvalue) (.y _returnvalue) (.z _returnvalue)))
  (bind _move (Timeline|Timeline_1 PlayFromStart)
    (:Update
      (Transformation|SetWorldLocation (Variables|Default|GetSphere) (Math|Vector|Lerp(Vector) (Variables|Default|GetStart2) (Variables|Default|GetEnd2) _move) false false))
    (:Finished
      (bind _move_2 (Timeline|Timeline_2 ReverseFromEnd)
        (:Update
          (Transformation|SetWorldLocation (Variables|Default|GetSphere) (Math|Vector|Lerp(Vector) (Variables|Default|GetStart2) (Variables|Default|GetEnd2) _move_2) false false))
        (:Finished
          (Timeline|Timeline_1 PlayFromStart))))))

(event Custom|CustomEvent_1
  (bind _sphere2 (Variables|Default|GetSphere2))
  (bind _returnvalue (Transformation|GetWorldLocation _sphere2))
  ;[1 1 1] Comment
  (bind _output_get (Variables|Default|SetStart1 (Math|Vector|MakeVector (.x _returnvalue) 6.7e+02 (.z _returnvalue))))
  (Development|PrintString (Utilities|String|ToString(Vector) _output_get))
  (Variables|Default|SetEnd1 (Math|Vector|MakeVector (.x _returnvalue) (.y _returnvalue) (.z _returnvalue)))
  (bind _move (Timeline|Timeline_3 PlayFromStart)
    (:Update
      (Transformation|SetWorldLocation (Variables|Default|GetSphere2) (Math|Vector|Lerp(Vector) (Variables|Default|GetStart1) (Variables|Default|GetEnd1) _move) false false))
    (:Finished
      (bind _move_2 (Timeline|Timeline_4 ReverseFromEnd)
        (:Update
          (Transformation|SetWorldLocation (Variables|Default|GetSphere2) (Math|Vector|Lerp(Vector) (Variables|Default|GetStart1) (Variables|Default|GetEnd1) _move_2) false false))
        (:Finished
          (Timeline|Timeline_3 PlayFromStart))))))

(event Collision|EventHit
  (params (MyComp :type Primitive%20Component%20Object%20Reference) (Other :type Actor%20Object%20Reference) (OtherComp :type Primitive%20Component%20Object%20Reference) (bSelfMoved :type Boolean) (HitLocation :type Vector :default "0, 0, 0") (HitNormal :type Vector :default "0, 0, 0") (NormalImpulse :type Vector :default "0, 0, 0") (Hit :type Hit%20Result%20Structure%20%28by%20ref%29))
  (if (== MyComp (Variables|Default|GetIsRed))
    (for _array_element (Variables|Default|GetTargets)
      (Rendering|Material|SetMaterial _array_element 0 "/Game/FPWeapon/Materials/BaseMaterial.BaseMaterial"))
    (bind _output_get (Variables|Default|SetIsRedNew (.OutItem (Utilities|Array|Random (Variables|Default|GetTargets)))))
    (if (!= _output_get (Variables|Default|GetIsRed))
      _
      (else
        (while (== _output_get (Variables|Default|GetIsRed))
          (Variables|Default|SetIsRedNew (.OutItem (Utilities|Array|Random (Variables|Default|GetTargets)))))))
    (Rendering|Material|SetMaterial _output_get 0 "/Game/Own/Material/M_Red.M_Red")
    (Variables|Default|SetIsRed _output_get)
    (bind _returnvalue (Actor|GetActorOfClass "/Game/Own/Widgets/BP_Spawn_ScoreCounter1.BP_Spawn_ScoreCounter1_C"))
    (bind _aswbp_score_counter (Utilities|Casting|CastToWBP_ScoreCounter (UserInterface|GetWidget (Variables|/Game/Own/Widgets/BP_Spawn_ScoreCounter1.BP_Spawn_ScoreCounter1_C|GetWidget _returnvalue))))
    (Default|Counter+ _aswbp_score_counter)
    (bind _output_get_2 (Variables|Default|SetScoreCounter (+ (Variables|Default|GetScoreCounter) 1)))
    (Development|PrintString (Utilities|String|ToString(Integer) _output_get_2))
    (if (== (Variables|Default|GetScoreCounter) 15)
      (for _array_element_2 (Variables|Default|GetTargets)
        (Actor|DestroyActor))
      (bind _returnvalue_2 (Actor|GetActorOfClass "/Game/Own/Widgets/BP_Spawn_TimeCounter1.BP_Spawn_TimeCounter1_C"))
      (bind _aswbp_time_counter (Utilities|Casting|CastToWBP_TimeCounter (UserInterface|GetWidget (Variables|/Game/Own/Widgets/BP_Spawn_TimeCounter1.BP_Spawn_TimeCounter1_C|GetWidget _returnvalue_2))))
      (Variables|/Game/Own/Widgets/WBP_TimeCounter.WBP_TimeCounter_C|SetGameWon_0 _aswbp_time_counter true)
      (Game|SpawnActorfromClass "/Game/Own/Blueprint/BP_Restart.BP_Restart_C" (Variables|Default|GetSpawn%20Transform) "Undefined" "MultiplyWithRoot" 0 0))
    (else
      (bind _output_get_3 (Variables|Default|SetScoreCounter (- (Variables|Default|GetScoreCounter) 1)))
      (Development|PrintString (Utilities|String|ToString(Integer) _output_get_3))
      (bind _returnvalue_3 (Actor|GetActorOfClass "/Game/Own/Widgets/BP_Spawn_ScoreCounter1.BP_Spawn_ScoreCounter1_C"))
      (bind _aswbp_score_counter_2 (Utilities|Casting|CastToWBP_ScoreCounter (UserInterface|GetWidget (Variables|/Game/Own/Widgets/BP_Spawn_ScoreCounter1.BP_Spawn_ScoreCounter1_C|GetWidget _returnvalue_3))))
      (Default|Counter- _aswbp_score_counter_2))))

(event EventBeginPlay
  (CallFunction|MovingTargets)
  (CallFunction|CustomEvent)
  (CallFunction|CustomEvent1)
  (CallFunction|CustomEvent2))

(fn ConstructionScript)