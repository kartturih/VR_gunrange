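; VR push button that starts a timed static-target round when overlapped.
; The first overlap spawns a five-second countdown with sound and removes the button text.
; A press by VRPawn lowers the button, calls countdown destruction, waits five seconds, then starts BP_TargetSphere targets and the time-counter widget's timer.
; ResetButton raises the button and clears IsPressed, but leaves the DoOnce gates on countdown and round start closed.
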(event OnComponentBeginOverlap(Collision)
  (params (OverlappedComponent :type Primitive%20Component%20Object%20Reference) (OtherActor :type Actor%20Object%20Reference) (OtherComp :type Primitive%20Component%20Object%20Reference) (OtherBodyIndex :type Integer) (bFromSweep :type Boolean) (SweepResult :type Hit%20Result%20Structure%20%28by%20ref%29))
  (CallFunction|ButtonPressed)
  (Utilities|FlowControl|DoOnce false
    (:Completed
      (Game|SpawnActorfromClass "/Game/Own/Widgets/BP_Spawn_CountdownTime.BP_Spawn_CountdownTime_C" (Variables|Default|GetSpawnCountdownTime) "Undefined" "MultiplyWithRoot" 0 0)
      (Audio|PlaySound2D "/Game/Own/Sounds/Countdown_5_seconds_timer.Countdown_5_seconds_timer" 1.0 1.0 0.0 0 0)
      (bind _returnvalue (Actor|GetActorOfClass "/Game/Own/Widgets/BP_Spawn_ButtonText.BP_Spawn_ButtonText_C"))
      (Default|DestoryButtonText _returnvalue))))

(event Custom|Reset%20Button
  (bind _button (Variables|Default|GetButton))
  (bind _returnvalue (Transformation|GetRelativeTransform _button))
  (Variables|Default|SetIsPressed false)
  (Components|MoveComponentTo _button (+ (.location _returnvalue) "0.000000,0.000000,15.000000") (.rotation _returnvalue) false false 0.2 false))

(event Custom|Button%20Pressed
  (bind _button (Variables|Default|GetButton))
  (bind _returnvalue (Transformation|GetRelativeTransform _button))
  (if (not (Variables|Default|GetIsPressed))
    (Variables|Default|SetIsPressed true)
    (Utilities|Casting|CastToVRPawn (stale OnComponentBeginOverlap(Collision) OtherActor))
    (Components|MoveComponentTo _button (- (.location _returnvalue) "0.000000,0.000000,15.000000") (.rotation _returnvalue) false false 0.2 false)
    (bind _returnvalue_2 (Actor|GetActorOfClass "/Game/Own/Widgets/BP_Spawn_CountdownTime.BP_Spawn_CountdownTime_C"))
    (Default|DestoryCountdown _returnvalue_2)
    (Utilities|FlowControl|Delay 5.0)
    ;[1 1 1] Start static targets
    (bind _returnvalue_3 (Actor|GetActorOfClass "/Game/Own/Blueprint/BP_TargetSphere.BP_TargetSphere_C"))
    (Utilities|FlowControl|DoOnce false
      (:Completed
        (Default|StartTargets _returnvalue_3)
        ;[1 1 1] Start timer static targets
        (bind _returnvalue_4 (Actor|GetActorOfClass "/Game/Own/Widgets/BP_Spawn_TimeCounter.BP_Spawn_TimeCounter_C"))
        (bind _aswbp_time_counter (Utilities|Casting|CastToWBP_TimeCounter (UserInterface|GetWidget (Variables|/Game/Own/Widgets/BP_Spawn_TimeCounter.BP_Spawn_TimeCounter_C|GetWidget _returnvalue_4))))
        (Default|StartTimer _aswbp_time_counter)))))

(fn ConstructionScript)